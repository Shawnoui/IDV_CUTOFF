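; BP_Pawn is a player camera pawn with smoothed panning, yaw rotation and spring arm zoom.
; Axis inputs update desired zoom, rotation and location, with zoom clamped to a range and movement following the actor's forward and right vectors.
; BeginPlay seeds the desired transform from the actor, and Tick interpolates arm length, location and rotation toward those targets using a shared interpolation speed.
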(event EventTick
  (params (DeltaSeconds :type Float%20%28single-precision%29))
  (bind _springarm (Variables|Default|GetSpringArm))
  (bind _interp_speed (Variables|Default|GetInterp_Speed))
  ;[1 1 1] Event Tick
  (Variables|/Script/Engine.SpringArmComponent|SetTargetArmLength _springarm (Math|Interpolation|FInterpTo (Variables|/Script/Engine.SpringArmComponent|GetTargetArmLength _springarm) (Variables|Default|GetZoom_Desired) DeltaSeconds _interp_speed))
  (Transformation|SetActorLocation (Math|Interpolation|VInterpTo (Transformation|GetActorLocation) (Variables|Default|GetCamLoc_Desired) DeltaSeconds _interp_speed) false false)
  (Transformation|SetActorRotation (Math|Interpolation|RInterpTo (Transformation|GetActorRotation) (Variables|Default|GetCamRot_Desired) DeltaSeconds _interp_speed)))

(event EventBeginPlay
  ;[1 1 1] Set Base Location & Rotation
  (Variables|Default|SetCamLoc_Desired (Transformation|GetActorLocation))
  (Variables|Default|SetCamRot_Desired (Transformation|GetActorRotation)))

(event Input|AxisEvents|InputAxisInputAxis_Zoom
  (params (AxisValue :type Float%20%28single-precision%29))
  ;[1 1 1] Input Axis
  (Variables|Default|SetZoom_Desired (Math|Float|Clamp(Float) (+ (Variables|Default|GetZoom_Desired) (* AxisValue 8e+01)) 1e+02 5e+03)))

(event Input|AxisEvents|InputAxisInputAxis_Forward
  (params (AxisValue :type Float%20%28single-precision%29))
  ;[1 1 1] Input Axis
  (Variables|Default|SetCamLoc_Desired (+ (Variables|Default|GetCamLoc_Desired) (* (Transformation|GetActorForwardVector) (* AxisValue 8e+01)))))

(event Input|AxisEvents|InputAxisInputAxis_Right
  (params (AxisValue :type Float%20%28single-precision%29))
  ;[1 1 1] Input Axis
  (Variables|Default|SetCamLoc_Desired (+ (Variables|Default|GetCamLoc_Desired) (* (Transformation|GetActorRightVector) (* AxisValue 8e+01)))))

(event Input|AxisEvents|InputAxisInputAxis_Rotation
  (params (AxisValue :type Float%20%28single-precision%29))
  ;[1 1 1] Input Axis
  (Variables|Default|SetCamRot_Desired (Math|Rotator|CombineRotators (Variables|Default|GetCamRot_Desired) (Math|Rotator|MakeRotator 0.0 0.0 AxisValue))))

(fn ConstructionScript)