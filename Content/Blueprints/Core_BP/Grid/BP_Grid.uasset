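; BP_Grid builds a tile grid around the actor in its construction script, as instanced static meshes styled per shape from DT_GridShapeData.
; SpawnGrid snaps the center to tile size, derives the bottom-left corner, and can sphere-trace each tile for height and type, omitting unwalkable ones.
; Overlapping BP_GridModifier actors set tile type.
; Helpers convert cursor hits, with a grid-plane intersection fallback, into tile indices.
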(event EventBeginPlay)

(event Collision|EventActorBeginOverlap
  (params (OtherActor :type Actor%20Object%20Reference)))

(event EventTick
  (params (DeltaSeconds :type Float%20%28single-precision%29)))

(fn ConstructionScript
  (CallFunction|SpawnGrid (Transformation|GetActorLocation) (Variables|Default|GetGridTileSize) (Variables|Default|GetGridTileCount) (Variables|Default|GetGridShape) true))

(fn SpawnGrid
  (params (CenterLocation :type Vector) (TileSize :type Vector) (TileCount :type Vector%202D%20Structure) (Shape :type E_GridShape%20Enum :default "NewEnumerator1") (UseEnvironment :type Boolean))
  (bind (_bottomleft _center) (CallFunction|CalculateCenter&BottomLeftLoc))
  (bind _instancedstaticmesh (Variables|Default|GetInstancedStaticMesh))
  (Variables|Default|SetGridCenterLocation CenterLocation)
  (Variables|Default|SetGridTileSize TileSize)
  (Variables|Default|SetGridShape Shape)
  (Variables|Default|SetGridTileCount (Math|Vector2D|MakeVector2D (Math|Conversions|ToFloat(Integer) (Math|Float|Round (.x (Variables|Default|GetGridTileCount)))) (Math|Conversions|ToFloat(Integer) (Math|Float|Round (.y (Variables|Default|GetGridTileCount))))))
  (Components|InstancedStaticMesh|ClearInstances (Variables|Default|GetInstancedStaticMesh))
  (bind _returnvalue (CallFunction|GetCurrentShapeData))
  (Components|StaticMesh|SetStaticMesh _instancedstaticmesh (.FlatMesh (Utilities|Struct|BreakS_GridShapeData _returnvalue)))
  (Rendering|Material|SetMaterial _instancedstaticmesh 0 (.FlatBorderMat (Utilities|Struct|BreakS_GridShapeData _returnvalue)))
  (Variables|Default|SetGridCenterLocation _center)
  (Variables|Default|SetGridBottomLeftCorner _bottomleft)
  (for _index (range 0 (Math|Float|Round (.x (Variables|Default|GetGridTileCount))))
    (LocalVariables|SetX _index)
    (for _index_2 (range 0 (Math|Float|Round (.y (Variables|Default|GetGridTileCount))))
      (LocalVariables|SetY _index_2)
      (bind _returnvalue_2 (CallFunction|GetCurrentShapeData))
      (LocalVariables|SetTileTransform (Math|Transform|MakeTransform (+ (Variables|Default|GetGridBottomLeftCorner) (* (Variables|Default|GetGridTileSize) (Math|Vector|MakeVector (LocalVariables|GetX) (LocalVariables|GetY) 0.0))) "0, 0, 0" (/ (Variables|Default|GetGridTileSize) (.MeshSize (Utilities|Struct|BreakS_GridShapeData _returnvalue_2)))))
      (if UseEnvironment
        (bind (_outlocation _tiletype) (CallFunction|TraceforGround (.location (LocalVariables|GetTileTransform))))
        (if (CallFunction|IsTileTypeWalkable _tiletype)
          (LocalVariables|SetTileTransform (Math|Transform|MakeTransform _outlocation (.rotation (LocalVariables|GetTileTransform)) (.scale (LocalVariables|GetTileTransform))))
          (Components|InstancedStaticMesh|AddInstance (Variables|Default|GetInstancedStaticMesh) (LocalVariables|GetTileTransform) true))
        (else
          (Components|InstancedStaticMesh|AddInstance (Variables|Default|GetInstancedStaticMesh) (LocalVariables|GetTileTransform) true))))))

(fn GetCurrentShapeData
  (bind _gridshape (Variables|Default|GetGridShape))
  (bind _returnvalue (Utilities|String|EnumtoString _gridshape))
  (bind _returnvalue_2 (Utilities|GetDataTableRow "/Game/Blueprints/Core_BP/Grid/DT_GridShapeData.DT_GridShapeData" (Utilities|String|StringToName _returnvalue))
    (:then
      _)
    (:RowNotFound
      (Development|PrintString (Utilities|String|Append "Error - Row Not Found - " _returnvalue) true true "(R=1.000000,G=0.000000,B=0.000000,A=1.000000)" 5.0)))
  (return _returnvalue_2))

(fn CalculateCenter&BottomLeftLoc
  (bind _gridtilecount (Variables|Default|GetGridTileCount))
  (LocalVariables|SetC (CallFunction|SnapVectortoVector (Variables|Default|GetGridCenterLocation) (Variables|Default|GetGridTileSize)))
  (return (- (Variables|Default|GetGridCenterLocation) (Math|Conversions|ToVector(Vector2D) (* (/ (- (Variables|Default|GetGridTileCount) (Math|Vector2D|MakeVector2D (Math|Float|SelectFloat 0.0 1.0 (CallFunction|IsFloatEven? (.x _gridtilecount))) (Math|Float|SelectFloat 0.0 1.0 (CallFunction|IsFloatEven? (.y _gridtilecount))))) 2.0) (Math|Conversions|ToVector2D(Vector) (Variables|Default|GetGridTileSize))))) (LocalVariables|GetC)))

(fn TraceforGround
  (params (Location :type Vector))
  (LocalVariables|SetRadius (/ (.x (Variables|Default|GetGridTileSize)) 3.0))
  (bind _outhits (Collision|MultiSphereTraceByChannel (+ Location "") (+ Location "") (LocalVariables|GetRadius) "TraceTypeQuery3" false 0 "ForDuration"))
  (if (> (Utilities|Array|Length _outhits) 0)
    (LocalVariables|SetRetType "NewEnumerator1")
    (for _array_element _outhits
      (bind _asbp_grid_modifier (Utilities|Casting|CastToBP_GridModifier (.HitActor (Collision|BreakHitResult _array_element)))
        (:then
          (LocalVariables|SetRetType (Variables|/Game/Blueprints/Core_BP/Grid/BP_GridModifier.BP_GridModifier_C|GetType _asbp_grid_modifier)))
        (:CastFailed
          (LocalVariables|SetRetZ (Math|Float|SnapToGrid(Float) (.Z (Math|Vector|BreakVector (.Location (Collision|BreakHitResult _array_element)))) (.z (Variables|Default|GetGridTileSize)))))))
    (return (Math|Vector|MakeVector (.x Location) (.y Location) (LocalVariables|GetRetZ)) (LocalVariables|GetRetType))
    (else
      (return Location "NewEnumerator0"))))

(fn GetCursorLocation
  (params (PlayerIndex :type Integer))
  (bind _returnvalue (Game|GetPlayerController PlayerIndex))
  (bind _gridcenterlocation (Variables|Default|GetGridCenterLocation))
  (bind (_hitresult _returnvalue_2) (Game|Player|GetHitResultUnderCursorbyChannel _returnvalue "TraceTypeQuery4" false))
  (bind (_worldlocation _worlddirection) (Game|Player|ConvertMouseLocationToWorldSpace _returnvalue))
  (bind _returnvalue_3 (Class|KismetMathLibrary|MakePlanefromPointandNormal _gridcenterlocation "0.000000,0.000000,1.000000"))
  (bind _returnvalue_4 (* _worlddirection 99999.0))
  (bind _returnvalue_5 (+ _worldlocation _returnvalue_4))
  (bind (_t _intersection _returnvalue_6) (Class|KismetMathLibrary|LinePlaneIntersection _worldlocation _returnvalue_5 _returnvalue_3))
  (if _returnvalue_2
    (return (.Location (Collision|BreakHitResult _hitresult)))
    (elif _returnvalue_6
      (return _intersection)
      (else
        (return "-999.000000,-999.000000,-999.000000")))))

(fn GetTileIndexfromWLoc
  (params (Location :type Vector))
  (LocalVariables|SetLocationOnGrid (- Location (Variables|Default|GetGridBottomLeftCorner)))
  (switch Utilities|FlowControl|Switch|SwitchonE_GridShape (Variables|Default|GetGridShape)
    (:NewEnumerator1
      (return (Utilities|Struct|MakeIntPoint -999 -999)))
    (:NewEnumerator2
      (LocalVariables|SetSnapLocationOnGrid (Math|Conversions|ToVector2D(Vector) (CallFunction|SnapVectortoVector (LocalVariables|GetLocationOnGrid) (Variables|Default|GetGridTileSize))))
      (return (Class|KismetMathLibrary|ToIntPoint(Vector2D) (/ (LocalVariables|GetSnapLocationOnGrid) (Math|Conversions|ToVector2D(Vector) (Variables|Default|GetGridTileSize))))))
    (:NewEnumerator3
      (LocalVariables|SetSnapLocationOnGrid (Math|Conversions|ToVector2D(Vector) (CallFunction|SnapVectortoVector (LocalVariables|GetLocationOnGrid) (Variables|Default|GetGridTileSize))))
      (return (Class|KismetMathLibrary|ToIntPoint(Vector2D) (/ (LocalVariables|GetSnapLocationOnGrid) (Math|Conversions|ToVector2D(Vector) (Variables|Default|GetGridTileSize))))))))

(fn GetTileIndexUnderCursor
  (params (PlayerIndex :type Integer))
  (bind _location (CallFunction|GetCursorLocation PlayerIndex))
  (bind _index (CallFunction|GetTileIndexfromWLoc _location))
  (return _index))

(fn IsTileTypeWalkable
  (params (Type :type E_TileType%20Enum :default "NewEnumerator0"))
  (return (not (Utilities|Array|ContainsItem (Utilities|Array|MakeArray "NewEnumerator0" "NewEnumerator2") Type))))