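; BP_CoreUnit is the logical unit actor, holding health and damage and offering move, attack and die events.
; On BeginPlay it spawns four BP_VisualUnit actors at fixed offsets, storing itself as their parent and as the CoreUnit key in their blackboards.
; Incoming damage lowers health until Die destroys the core actor alone.
; MoveTo sets location directly without sweep, and Attack applies damage to the given target.
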(event Custom|MoveTo
  (params (Position :type Vector))
  (Transformation|SetActorLocation Position false false))

(event Custom|Attack
  (params (Target :type BP%20Core%20Unit%20Object%20Reference))
  (Game|Damage|ApplyDamage Target (Variables|Default|GetDamages) 0 self))

(event Custom|OnTakeAnyDamage_Event
  (params (DamagedActor :type Actor%20Object%20Reference) (Damage :type Float%20%28single-precision%29) (DamageType :type Damage%20Type%20Object%20Reference) (InstigatedBy :type Controller%20Object%20Reference) (DamageCauser :type Actor%20Object%20Reference))
  (bind _output_get (Variables|Default|SetHealth (- (Variables|Default|GetHealth) Damage)))
  (if (<= _output_get 0.0)
    (CallFunction|Die)))

(event Custom|Die
  (Actor|DestroyActor))

(event EventBeginPlay
  (EventDispatchers|AssignOnTakeAnyDamage (delegate Custom|OnTakeAnyDamage_Event))
  (Utilities|VisualUnitSpawner "150.000000,0.000000,0.000000")
  (Utilities|VisualUnitSpawner "-150.000000,0.000000,0.000000")
  (Utilities|VisualUnitSpawner "150.000000,150.000000,0.000000")
  (Utilities|VisualUnitSpawner "-150.000000,-150.000000,0.000000"))

(event Collision|EventActorBeginOverlap
  (params (OtherActor :type Actor%20Object%20Reference)))

(event EventTick
  (params (DeltaSeconds :type Float%20%28single-precision%29)))

(fn ConstructionScript)