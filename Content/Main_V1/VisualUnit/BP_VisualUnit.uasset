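; BP_VisualUnit is an AI-controlled unit that runs the BT_Vunit behavior tree and labels itself with its object name.
; On BeginPlay it starts the tree if its controller is an AIController.
; Every Tick it draws the name as a magenta debug string above the actor, shifted along Y by name length, apparently to center it.
; An AIMoveTo node is left unconnected.
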(event EventBeginPlay
  (bind _asaicontroller (Utilities|Casting|CastToAIController (Pawn|GetController)))
  (AI|RunBehaviorTree _asaicontroller "/Game/Main_V1/VisualUnit/BT_Vunit.BT_Vunit"))

(event Collision|EventActorBeginOverlap
  (params (OtherActor :type Actor%20Object%20Reference)))

(event EventTick
  (params (DeltaSeconds :type Float%20%28single-precision%29))
  (bind _self self)
  (bind _returnvalue (Utilities|GetObjectName _self))
  (Rendering|Debug|DrawDebugString (+ (+ (Transformation|GetActorLocation) "0.000000,0.000000,100.000000") (* "0.000000,-5.000000,0.000000" (Utilities|String|Len _returnvalue))) _returnvalue 0 "(R=1.000000,G=0.000000,B=0.970430,A=1.000000)"))

(fn ConstructionScript)